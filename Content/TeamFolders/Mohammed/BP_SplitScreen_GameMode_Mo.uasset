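; Split-screen game mode that spawns a local player for every connected input device at BeginPlay.
; ChoosePlayerStart gives each player the PlayerStart tagged with the current PlayerController count minus one, so spawn points follow join order.
; Handling of device connection changes, including removing players on disconnect, is deprecated and left unwired.
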(event `self.ReceiveBeginPlay`
  (`|ExecutionSequence`
    (:`then_0`
      (bind _outinputdevices (`InputDeviceLibrary.GetAllInputDevices`))
      (for (_ _array_index) _outinputdevices
        (`GameplayStatics.CreatePlayer` _array_index)))))

(event `OnInputDeviceConnectionChange_Event`
  (params (NewConnectionState :type "EInputDeviceConnectionState Enum" :default "Invalid") (PlatformUserId :type "PlatformUserId Structure") (InputDeviceId :type "InputDeviceId Structure"))
  ; Deprecated
)

(event `ConnectExistingDevices`
  ; Deprecated
  (bind _outinputdevices (`InputDeviceLibrary.GetAllInputDevices`))
  (for (_ _array_index) _outinputdevices
    (if (!= _array_index 0)
      (`GameplayStatics.CreatePlayer` _array_index))))

(fn `ChoosePlayerStart`
  (params (Player :type "Controller Object Reference"))
  (returns (ReturnValue :type "Actor Object Reference"))
  (`parent.ChoosePlayerStart` Player)
  (bind _outactors (`GameplayStatics.GetAllActorsOfClass` "/Script/Engine.PlayerController"))
  (bind _outactors_2 (`GameplayStatics.GetAllActorsOfClassWithTag` "/Script/Engine.PlayerStart" (`KismetStringLibrary.Conv_StringToName` (`KismetStringLibrary.Conv_IntToString` (- (`KismetArrayLibrary.Array_Length` _outactors) 1)))))
  (return (`|GetArrayItem` _outactors_2)))

(fn `UserConstructionScript`)