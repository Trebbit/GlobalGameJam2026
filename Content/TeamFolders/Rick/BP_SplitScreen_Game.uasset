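; Split-screen game mode that spawns a local player for every input device found at BeginPlay and gives each a WBP_PlayerHUD on their own screen.
; ChoosePlayerStart picks the PlayerStart tagged with the current player controller count minus one.
; A handler removes disconnected non-zero devices' players and pawns, but its binding and the ConnectExistingDevices call are left unwired, as is player creation on connect.
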(event `self.ReceiveBeginPlay`
  (bind _outinputdevices (`InputDeviceLibrary.GetAllInputDevices`))
  (for (_ _array_index) _outinputdevices
    (bind _returnvalue (`GameplayStatics.CreatePlayer` _array_index))
    (bind _returnvalue_2 (`|CreateWidget` "/Game/TeamFolders/Rick/WBP_PlayerHUD.WBP_PlayerHUD_C" _returnvalue))
    (if (`KismetSystemLibrary.IsValid` _returnvalue_2)
      (`UserWidget.AddToPlayerScreen` _returnvalue_2 0)
      (else
        (`KismetSystemLibrary.PrintString` "Hello")))))

(event `OnInputDeviceConnectionChange_Event`
  (params (NewConnectionState :type "EInputDeviceConnectionState Enum" :default "Invalid") (PlatformUserId :type "PlatformUserId Structure") (InputDeviceId :type "InputDeviceId Structure"))
  (bind _returnvalue (`KismetStringLibrary.Conv_InputDeviceIdToString` InputDeviceId))
  (`KismetSystemLibrary.PrintText` (`KismetTextLibrary.Conv_StringToText` _returnvalue))
  (if (!= (`KismetStringLibrary.Conv_StringToInt` _returnvalue) 0)
    (switch `EInputDeviceConnectionState` NewConnectionState
      (:`Disconnected`
        (bind _returnvalue_2 (`InputDeviceLibrary.GetPlayerControllerFromInputDevice` InputDeviceId))
        (`GameplayStatics.RemovePlayer` _returnvalue_2 true)))))

(event `ConnectExistingDevices`
  (bind _outinputdevices (`InputDeviceLibrary.GetAllInputDevices`))
  (for (_ _array_index) _outinputdevices
    (if (!= _array_index 0)
      (bind _returnvalue (`GameplayStatics.CreatePlayer` _array_index))
      (bind _returnvalue_2 (`|CreateWidget` "/Game/TeamFolders/Rick/WBP_PlayerHUD.WBP_PlayerHUD_C" _returnvalue))
      (if (`KismetSystemLibrary.IsValid` _returnvalue_2)
        (`UserWidget.AddToPlayerScreen` _returnvalue_2 0)
        (else
          (`KismetSystemLibrary.PrintString` "Hello"))))))

(fn `ChoosePlayerStart`
  (params (Player :type "Controller Object Reference"))
  (returns (ReturnValue :type "Actor Object Reference"))
  (`parent.ChoosePlayerStart` Player)
  (bind _outactors (`GameplayStatics.GetAllActorsOfClass` "/Script/Engine.PlayerController"))
  (bind _outactors_2 (`GameplayStatics.GetAllActorsOfClassWithTag` "/Script/Engine.PlayerStart" (`KismetStringLibrary.Conv_StringToName` (`KismetStringLibrary.Conv_IntToString` (- (`KismetArrayLibrary.Array_Length` _outactors) 1)))))
  (return (`|GetArrayItem` _outactors_2)))

(fn `UserConstructionScript`)